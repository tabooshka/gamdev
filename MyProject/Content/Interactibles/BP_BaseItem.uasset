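; BP_BaseItem is a pickup item that players collect through an Interaction event, carrying its data in an ItemInfo struct.
; On interaction, it checks that the instigator has inventory space, passes ItemInfo to the instigator's PickupMessage, then destroys itself.
; The construction script only calls its parent; a disconnected node that would write the item's own class into ItemInfo never runs.
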(event EventInteraction
  (params (Instigator :type CH%20Mycharacter%20Object%20Reference))
  (if (Default|HasSpaceinInventory Instigator)
    (Class|BPIInteract|Pickup(Message) Instigator (Variables|Default|GetItem_info))
    (Actor|DestroyActor)))

(fn ConstructionScript
  (|CallParentFunction))