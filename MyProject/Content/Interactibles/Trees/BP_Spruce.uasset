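; Choppable spruce tree that shows a deepening cut as it takes hits, then falls on the fifth.
; An overlap zone prompts the player and gates point damage, which steps cut depth in a dynamic wood material displaced around a hit-location component.
; The final hit swaps the intact mesh for a stump and a physics-simulated falling top.
; The construction script applies the same material parameters from editable values, previewing the cut.
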(event OnComponentBeginOverlap(ActiveZone1)
  (params (OverlappedComponent :type Primitive%20Component%20Object%20Reference) (OtherActor :type Actor%20Object%20Reference) (OtherComp :type Primitive%20Component%20Object%20Reference) (OtherBodyIndex :type Integer) (bFromSweep :type Boolean) (SweepResult :type Hit%20Result%20Structure%20%28by%20ref%29))
  (if (not (Variables|Default|GetHit5Recieved))
    (Input|EnableInput (Game|GetPlayerController 0))
    (Variables|Default|SetZone1IsActive true)
    (Development|PrintString "Uderz w drzewo" true true "(R=1.000000,G=1.000000,B=0.000000,A=1.000000)")))

(event OnComponentEndOverlap(ActiveZone1)
  (params (OverlappedComponent :type Primitive%20Component%20Object%20Reference) (OtherActor :type Actor%20Object%20Reference) (OtherComp :type Primitive%20Component%20Object%20Reference) (OtherBodyIndex :type Integer))
  (Input|DisableInput (Game|GetPlayerController 0))
  (Variables|Default|SetZone1IsActive false))

(event Game|Damage|EventPointDamage
  (params (Damage :type Float%20%28single-precision%29) (DamageType :type Damage%20Type%20Object%20Reference) (HitLocation :type Vector :default "0, 0, 0") (HitNormal :type Vector :default "0, 0, 0") (HitComponent :type Primitive%20Component%20Object%20Reference) (BoneName :type Name :default "None") (ShotFromDirection :type Vector :default "0, 0, 0") (InstigatedBy :type Controller%20Object%20Reference) (DamageCauser :type Actor%20Object%20Reference) (HitInfo :type Hit%20Result%20Structure%20%28by%20ref%29))
  (bind _staticmesh (Variables|Default|GetStaticMesh))
  (bind _fallingtop (Variables|Default|GetFallingTop))
  (bind _cut_depth_location_1 (Variables|Default|GetCut%20Depth%20Location%201))
  (bind _woodmat (Variables|Default|GetWoodMat))
  (if (not (Variables|Default|GetHit5Recieved))
    (Components|Activation|Activate (Variables|Default|GetParticleSystem) true)
    (if (Variables|Default|GetZone1IsActive)
      (if (Variables|Default|GetHit1Recieved)
        (if (Variables|Default|GetHit2Recieved)
          (if (Variables|Default|GetHit3Recieved)
            (if (Variables|Default|GetHit4Recieved)
              (Variables|Default|SetHit5Recieved true)
              (else
                (Rendering|Material|SetScalarParameterValue _woodmat "CutDepth1" (* 12.0 _cut_depth_location_1) :!class /Script/Engine.MaterialInstanceDynamic)
                (Variables|Default|SetHit4Recieved true)))
            (else
              (Rendering|Material|SetScalarParameterValue _woodmat "CutDepth1" (* 6.0 _cut_depth_location_1) :!class /Script/Engine.MaterialInstanceDynamic)
              (Variables|Default|SetHit3Recieved true)))
          (else
            (Rendering|Material|SetScalarParameterValue _woodmat "CutDepth1" (* 3.0 _cut_depth_location_1) :!class /Script/Engine.MaterialInstanceDynamic)
            (Variables|Default|SetHit2Recieved true)))
        (else
          (Rendering|Material|SetScalarParameterValue _woodmat "CutDepth1" (* 1.0 _cut_depth_location_1) :!class /Script/Engine.MaterialInstanceDynamic)
          (Variables|Default|SetHit1Recieved true)))
      (Development|PrintString "Chop!")
      (if (Variables|Default|GetHit5Recieved)
        (Development|PrintString "TIMBER!!!" true true "(R=1.000000,G=0.000000,B=0.000000,A=1.000000)")
        (Rendering|SetVisibility _staticmesh false false)
        (Collision|SetCollisionEnabled _staticmesh "NoCollision")
        (Rendering|SetVisibility _fallingtop true false)
        (Rendering|SetVisibility (Variables|Default|GetStump) true false)
        (Physics|SetSimulatePhysics _fallingtop true)))))

(event EventBeginPlay
  (bind _staticmesh (Variables|Default|GetStaticMesh))
  (bind _returnvalue (Rendering|Material|CreateDynamicMaterialInstance _staticmesh 1 (Rendering|Material|GetMaterial _staticmesh 1) :!class /Script/Engine.PrimitiveComponent))
  (bind _output_get (Variables|Default|SetWoodMat _returnvalue))
  (Rendering|Material|SetVectorParameterValue _output_get "HitLocation1" (Math|Conversions|ToLinearColor(Vector) (Transformation|GetWorldLocation (Variables|Default|GetHitLocation1))) :!class /Script/Engine.MaterialInstanceDynamic)
  (Rendering|Material|SetScalarParameterValue _output_get "CutDepth1" 0.0 :!class /Script/Engine.MaterialInstanceDynamic)
  (Rendering|Material|SetScalarParameterValue _output_get "Displacement" 8.75 :!class /Script/Engine.MaterialInstanceDynamic)
  (Variables|Default|SetCut%20Depth%20Location%201 8.75))

(fn ConstructionScript
  (bind _staticmesh (Variables|Default|GetStaticMesh))
  (bind _cut_depth_location_1 (Variables|Default|GetCut%20Depth%20Location%201))
  (bind _returnvalue (Rendering|Material|CreateDynamicMaterialInstance _staticmesh 1 (Rendering|Material|GetMaterial _staticmesh 1) :!class /Script/Engine.PrimitiveComponent))
  (bind _output_get (Variables|Default|SetWoodMat _returnvalue))
  (Rendering|Material|SetVectorParameterValue _output_get "HitLocation1" (Math|Conversions|ToLinearColor(Vector) (Transformation|GetWorldLocation (Variables|Default|GetHitLocation1))) :!class /Script/Engine.MaterialInstanceDynamic)
  (Rendering|Material|SetScalarParameterValue _output_get "Displacement" (* _cut_depth_location_1 1.75) :!class /Script/Engine.MaterialInstanceDynamic)
  (Rendering|Material|SetScalarParameterValue _output_get "CutDepth1" (* _cut_depth_location_1 (Variables|Default|GetCDInfluence%201)) :!class /Script/Engine.MaterialInstanceDynamic))